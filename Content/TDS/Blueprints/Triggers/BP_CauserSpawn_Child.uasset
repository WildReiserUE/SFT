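; BP_CauserSpawn_Child is a one-shot trigger that activates its linked spawners when a Team1 player enters its collision component.
; On overlap it optionally shows a widget if IsCanShow is set, then calls SpawnMessage on each entry in Spawners, passing the player.
; It destroys itself after any player character overlap, so a player from another team consumes it without spawning, while other actors are ignored.
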(event `self.CollisionComponent.OnComponentBeginOverlap`
  (params (OverlappedComponent :type "PrimitiveComponent Object Reference") (OtherActor :type "Actor Object Reference") (OtherComp :type "PrimitiveComponent Object Reference") (OtherBodyIndex :type Integer) (bFromSweep :type Boolean) (SweepResult :type "HitResult Structure (by ref)"))
  (bind _spawners (`self.Spawners`))
  (bind _asbp_player_character (cast `/Game/TDS/Blueprints/Character/BP_PlayerCharacter` OtherActor))
  (if (`|EnumEquality` (`TDSCharacter.NewTeamID` _asbp_player_character) "Team_1")
    (if (`self.bIsCanShow`)
      (`self.TryToShowWidget` _asbp_player_character))
    (for (_array_element _array_index) _spawners
      (if (`KismetArrayLibrary.Array_IsValidIndex` _spawners _array_index)
        (message `/Game/TDS/Blueprints/Spawner/BP_InterfaceSpawner.Spawn` _array_element _asbp_player_character)))
    (`self.K2_DestroyActor`)
    (else
      (`self.K2_DestroyActor`))))

(fn `UserConstructionScript`
  (`parent.UserConstructionScript`))