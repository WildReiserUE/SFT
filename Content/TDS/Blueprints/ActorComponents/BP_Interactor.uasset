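; BP_Interactor is an actor component that makes its owning actor respond to mouse hover and clicks.
; On BeginPlay it binds the owner's cursor and click events, using the static mesh component or, failing that, a skeletal mesh component.
; Hovering toggles that mesh's custom depth rendering.
; Clicks fire the BPClicked dispatcher if either mesh reference is valid.
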(event `OnMouseStaticHover`
  (params (TouchedActor :type "Actor Object Reference"))
  (`PrimitiveComponent.SetRenderCustomDepth` (`self.MeshComp`) true))

(event `self.ReceiveBeginPlay`
  (bind _output_get (set `self.Owner` (`self.GetOwner`)))
  (add `Actor.OnClicked` _output_get (delegate `OnMouseClicked`))
  (bind _returnvalue (`Actor.GetComponentByClass` _output_get "/Script/Engine.StaticMeshComponent"))
  (`/Engine/EditorBlueprintResources/StandardMacros.IsValid` _returnvalue
    (:`Is Valid`
      (set `self.MeshComp` _returnvalue)
      (add `Actor.OnBeginCursorOver` _output_get (delegate `OnMouseStaticHover`))
      (add `Actor.OnEndCursorOver` _output_get (delegate `OnMouseStaticLeave`)))
    (:`Is Not Valid`
      (bind _returnvalue_2 (`Actor.GetComponentByClass` _output_get "/Script/Engine.SkeletalMeshComponent"))
      (`/Engine/EditorBlueprintResources/StandardMacros.IsValid` _returnvalue_2
        (:`Is Valid`
          (set `self.SkeletComp` _returnvalue_2)
          (add `Actor.OnBeginCursorOver` _output_get (delegate `OnMouseHover`))
          (add `Actor.OnEndCursorOver` _output_get (delegate `OnMouseLeave`)))))))

(event `OnMouseStaticLeave`
  (params (TouchedActor :type "Actor Object Reference"))
  (`PrimitiveComponent.SetRenderCustomDepth` (`self.MeshComp`) false))

(event `OnMouseHover`
  (params (TouchedActor :type "Actor Object Reference"))
  (`PrimitiveComponent.SetRenderCustomDepth` (`self.SkeletComp`) true))

(event `OnMouseLeave`
  (params (TouchedActor :type "Actor Object Reference"))
  (`PrimitiveComponent.SetRenderCustomDepth` (`self.SkeletComp`) false))

(event `OnMouseClicked`
  (params (TouchedActor :type "Actor Object Reference") (ButtonPressed :type "Key Structure" :default "None"))
  (`/Engine/EditorBlueprintResources/StandardMacros.IsValid` (`self.MeshComp`)
    (:`Is Valid`
      _)
    (:`Is Not Valid`
      (`/Engine/EditorBlueprintResources/StandardMacros.IsValid` (`self.SkeletComp`)
        (:`Is Valid`
          _))))
  (`self.BPClicked`))