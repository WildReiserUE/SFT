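; BP_GS_World is a world Blueprint, likely a game state, that tracks player lives and decides whether the player can respawn.
; CanPlayerRespawn lets the first spawn through without cost, clearing FirstStart, then deducts a life on each later call.
; It returns success while lives stay non-negative, along with the current stage, or the first enum entry once lives are already negative.
; GetPlayerCanRestart simply returns the FirstStart flag.
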(fn `CanPlayerRespawn`
  (returns (bIsSuccess :type Boolean) (E_CurrentStage :type "/Game/TDS/Blueprints/Game/E_LevelStage Enum"))
  (bind _playerlives (`self.PlayerLives`))
  (bind _returnvalue (>= _playerlives 0))
  (if (and (`self.bFirstStart`) _returnvalue)
    (bind _output_get (set `self.bFirstStart` (`self.bFirstStart`)))
    (if _output_get
      (set `self.bFirstStart` false)
      (return _returnvalue (`self.E_CurrentStage`))
      (else
        _))
    (elif _returnvalue
      _
      (else
        (return false "NewEnumerator0"))))
  (`/Engine/EditorBlueprintResources/StandardMacros.DecrementInt` _playerlives
    (:`  `
      (return _returnvalue (`self.E_CurrentStage`)))))

(fn `GetPlayerCanRestart`
  (returns (bCanRestart :type Boolean))
  (return (`self.bFirstStart`)))

(fn `UserConstructionScript`)