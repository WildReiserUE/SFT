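; Player controller for the 03World map that owns the main game HUD, pause menu and game-over screen.
; On begin play and restart it respawns through the game mode, restores saved weapons and diary from player state, creates the HUD and binds character events.
; Those events update the weapon panel, ammo counts, diary and tutorial popups.
; Death offers restart or main menu, while Tab or Escape opens the pause menu.
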(event `Again`
  ;[0 1 0] Начало
  (`GameplayStatics.PushSoundMixModifier` null :!label _label)
  (bind _asbp_gm_03world (cast `/Game/TDS/Blueprints/Game/BP_GM_03World` (`GameplayStatics.GetGameMode`)))
  (bind _success (`/Game/TDS/Blueprints/Game/BP_GM_03World.TryToRespawn` _asbp_gm_03world))
  (if _success
    (bind _asbp_player_character (cast `/Game/TDS/Blueprints/Character/BP_PlayerCharacter` (`GameplayStatics.GetPlayerPawn` 0)))
    (add `TDSCharacter.OnChangeStory` _asbp_player_character (delegate `OnChangeStory_Event_0`))
    (bind _output_get (set `self.As BP Player Character` _asbp_player_character))
    (set `TDSCharacter.bIsALive` true _output_get)
    (bind _asbp_ps_world (cast `/Game/TDS/Blueprints/Game/BP_PS_World` (`self.PlayerState`)))
    (bind _playerinventory (`TDSCharacter.PlayerInventory` _output_get))
    (set `TDSInventoryComponent.WeaponInventory` (`/Game/TDS/Blueprints/Game/BP_PS_World.SavedWeapon Set` _asbp_ps_world) _playerinventory)
    (set `TDSInventoryComponent.DiaryArray` (`/Game/TDS/Blueprints/Game/BP_PS_World.SavesTDSDiary` _asbp_ps_world) _playerinventory)
    (bind _gamewidget (`self.CreateGameWidget` self))
    (set `self.W_GameWidget` _gamewidget)
    (`self.BindEvents`)
    (add `Button.OnClicked` (`/Game/TDS/UI/UI_03_Game/WBP_TutorialDiary.Button_88` (`/Game/TDS/UI/UI_03_Game/W_GameMain.WBP_TutorialDiary` (`self.W_GameWidget`))) (delegate `OnClicked_Event_0`))
    (add `TDSInventoryComponent.OnPressed_T` (`TDSCharacter.PlayerInventory` (`self.As BP Player Character`)) (delegate `OnPressed_T`))
    (bind _returnvalue (`GameplayStatics.SetGamePaused` false))
    (set `self.bIsPaused` _returnvalue)))

(event `self.ReceiveBeginPlay`
  ;[0 1 0] Начало
  (goto _label))

(event `OnPressed_T`
  (bind _w_gamewidget (`self.W_GameWidget`))
  ;[0 1 0] Начало
  (if (not (`self.bIsFinishedTutorialTree`))
    (`/Game/TDS/UI/UI_03_Game/W_GameMain.OnShowMission` (`self.W_GameWidget`) "Сок дал побочный эффект: \"Медвежья сила\"")
    (set `self.bIsFinishedTutorialTree` true)
    (`KismetSystemLibrary.Delay` 2.0)
    (`/Game/TDS/UI/UI_03_Game/W_GameMain.OnCloseMission` _w_gamewidget)
    (`/Game/TDS/UI/UI_03_Game/W_GameMain.OnShowBearImage` _w_gamewidget)
    (`/Game/TDS/UI/UI_03_Game/W_GameMain.OnShowBottle` _w_gamewidget)))

(event `OnChangeStory_Event_0`
  ;[0 1 0] Начало
  (set `/Game/TDS/UI/UI_03_Game/W_GameMain.Index` 20 (`self.W_GameWidget`)))

(event `OnClicked_Event_0`
  (bind _w_gamewidget (`self.W_GameWidget`))
  ;[0 1 0] Начало
  (`GameplayStatics.SetGamePaused` false)
  (`UserWidget.PlayAnimation` _w_gamewidget (`/Game/TDS/UI/UI_03_Game/W_GameMain.A_CloseTutorial` _w_gamewidget) 0.0 1 "Forward" 1.0 false))

(event `ShowDeathWidget`
  (bind _wbp_gameover (`/Game/TDS/UI/UI_03_Game/W_GameMain.WBP_GameOver` (`self.W_GameWidget`)))
  ;[0 1 0] DEATH WIDGET
  (`Widget.SetVisibility` _wbp_gameover "Visible")
  (add `/Game/TDS/UI/UI_03_Game/WBP_GameOver.Click_Restart` _wbp_gameover (delegate `CustomEvent_1`))
  (add `/Game/TDS/UI/UI_03_Game/WBP_GameOver.Click_MainMenu` _wbp_gameover (delegate `CustomEvent_3`)))

(event `Key|Tab`
  (params (Key :type "Key Structure"))
  (bind _w_gamewidget (`self.W_GameWidget`))
  (bind _menu_box (`/Game/TDS/UI/UI_03_Game/W_GameMain.Menu_Box` _w_gamewidget))
  ;[1 1 0] GameMenu
  (:`Pressed`
    (bind _returnvalue (`GameplayStatics.SetGamePaused` true :!label _label_2))
    (bind _output_get (set `self.bIsPaused` _returnvalue))
    (if _output_get
      (add `/Game/TDS/UI/UI_03_Game/W_GameMain.Click_CloseMenu` _w_gamewidget (delegate `Click_CloseMenu_Event_0`))
      (add `/Game/TDS/UI/UI_03_Game/W_GameMain.Click_ExitToMainMenu` _w_gamewidget (delegate `Click_ExitToMainMenu_Event_0`))
      (if (`Widget.IsVisible` _menu_box)
        (`Widget.SetVisibility` _menu_box "Hidden" :!label _label_3)
        (else
          (`Widget.SetVisibility` _menu_box "Visible"))))))

(event `CustomEvent_3`
  ;[0 1 0] DEATH WIDGET
  (`GameplayStatics.OpenLevel` "StartMap"))

(event `Key|Escape` :paused true
  (params (Key :type "Key Structure"))
  ;[1 1 0] GameMenu
  (:`Pressed`
    (goto _label_2)))

(event `CustomEvent_1`
  ;[0 1 0] DEATH WIDGET
  (`Widget.RemoveFromParent` (`self.W_GameWidget`))
  (`self.UnPossess`)
  ;[1 1 0] TO DO
  (`self.Again`))

(event `Click_CloseMenu_Event_0`
  ;[1 1 0] GameMenu
  (`GameplayStatics.SetGamePaused` false)
  (goto _label_3))

(event `Click_ExitToMainMenu_Event_0`
  ;[1 1 0] GameMenu
  (`Widget.SetVisibility` (`/Game/TDS/UI/UI_03_Game/W_GameMain.Menu_Box` (`self.W_GameWidget`)) "Hidden")
  (`GameplayStatics.OpenLevel` "StartMap"))

(event `OnShow`
  ;[1 1 0] GameMenu
  (`/Game/TDS/UI/UI_03_Game/W_GameMain.OnShowDialog` (`self.W_GameWidget`)))

(event `BindEvents`
  (bind _as_bp_player_character (`self.As BP Player Character`))
  (bind _playerinventory (`TDSCharacter.PlayerInventory` (`self.As BP Player Character`)))
  ;[1 1 0] TODO - Update ammo - pickup
  (add `TDSPlayerStateComponent.OnPlayerDeath` (`TDSCharacter.PlayerStateInfo` _as_bp_player_character) (delegate `CustomEvent`))
  (add `TDSCharacter.OnPlayerWeaponSwitch` _as_bp_player_character (delegate `CustomEvent_2`))
  (add `TDSInventoryComponent.OnPlayerFindWeapon` _playerinventory (delegate `CustomEvent_4`))
  (add `TDSInventoryComponent.OnPlayerFindItem` _playerinventory (delegate `OnPlayerFindItem`))
  (add `TDSInventoryComponent.OnPlayerFindDiary` _playerinventory (delegate `OnPlayerFindDiary_Event_0`)))

(event `CustomEvent`
  ;[1 1 0] TODO - Update ammo - pickup
  (set `TDSCharacter.bIsALive` false (`self.As BP Player Character`))
  (`self.ShowDeathWidget`))

(event `CustomEvent_2`
  ;[1 1 0] TODO - Update ammo - pickup
  (add `TDSWeaponBase.OnWeaponFire` (`TDSCharacter.CurrentWeapon` (`self.As BP Player Character`)) (delegate `WeaponFire`))
  (`self.WeaponFire`))

(event `CustomEvent_4`
  (bind _playerinventory (`TDSCharacter.PlayerInventory` (`self.As BP Player Character`)))
  ;[1 1 0] TODO - Update ammo - pickup
  (`/Game/TDS/UI/UI_03_Game/W_WeaponPanel.FindWeapon` (`/Game/TDS/UI/UI_03_Game/W_GameMain.W_WeaponPanel` (`self.W_GameWidget`)) (`TDSInventoryComponent.WeaponInventory` _playerinventory))
  (add `TDSInventoryComponent.OnBulletsEnd` _playerinventory (delegate `OnBulletsEnd`)))

(event `OnBulletsEnd`
  (bind _as_bp_player_character (`self.As BP Player Character`))
  ;[1 1 0] TODO - Update ammo - pickup
  (`/Game/TDS/UI/UI_03_Game/W_WeaponPanel.CharacterShot` (`/Game/TDS/UI/UI_03_Game/W_GameMain.W_WeaponPanel` (`self.W_GameWidget`)) (`KismetArrayLibrary.Array_Find` (`TDSInventoryComponent.WeaponInventory` (`TDSCharacter.PlayerInventory` _as_bp_player_character)) (`GameplayStatics.GetObjectClass` (`TDSCharacter.CurrentWeapon` _as_bp_player_character))) 0))

(event `OnPlayerFindItem`
  ;[1 1 0] TODO - Update ammo - pickup
  (`/Game/TDS/UI/UI_03_Game/W_WeaponPanel.CharacterFindAmmo` (`/Game/TDS/UI/UI_03_Game/W_GameMain.W_WeaponPanel` (`self.W_GameWidget`))))

(event `WeaponFire`
  (bind _as_bp_player_character (`self.As BP Player Character`))
  (bind _playerinventory (`TDSCharacter.PlayerInventory` _as_bp_player_character))
  (bind _currentweapon (`TDSCharacter.CurrentWeapon` _as_bp_player_character))
  (bind _inventoryarray (`TDSInventoryComponent.InventoryArray` _playerinventory))
  ;[1 1 0] TODO - Update ammo - pickup
  (for (_array_element _array_index) _inventoryarray
    (if (`KismetArrayLibrary.Array_IsValidIndex` _inventoryarray _array_index)
      (bind (_id _count) (break `ItemSettings` _array_element))
      (if (== (`.BulletItemId` (break `WeaponSettings` (`TDSWeaponBase.WeaponInfo` _currentweapon))) _id)
        (`/Game/TDS/UI/UI_03_Game/W_WeaponPanel.CharacterShot` (`/Game/TDS/UI/UI_03_Game/W_GameMain.W_WeaponPanel` (`self.W_GameWidget`)) (`KismetArrayLibrary.Array_Find` (`TDSInventoryComponent.WeaponInventory` _playerinventory) (`GameplayStatics.GetObjectClass` _currentweapon)) _count)))))

(event `OnPlayerFindDiary_Event_0`
  ;[1 1 0] TODO - Update ammo - pickup
  (`/Game/TDS/UI/UI_03_Game/WBP_Diaryes.AddDiaryButton` (`/Game/TDS/UI/UI_03_Game/W_GameMain.WBP_Diaries` (`self.W_GameWidget`)) (`TDSInventoryComponent.DiaryArray` (`TDSCharacter.PlayerInventory` (`self.As BP Player Character`)))))

(fn `CreateGameWidget`
  (params (OwningPlayer :type "PlayerController Object Reference"))
  (returns (GameWidget :type "/Game/TDS/UI/UI_03_Game/W_GameMain Object Reference"))
  (bind _returnvalue (`|CreateWidget` "/Game/TDS/UI/UI_03_Game/W_GameMain.W_GameMain_C" OwningPlayer))
  (bind _output_get (set `self.W_GameWidget` _returnvalue))
  (`UserWidget.AddToViewport` _output_get 0)
  (return _output_get))

(fn `UserConstructionScript`)