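; Enemy spawner that populates a box volume with actors of a configurable enemy class when its Spawn event fires.
; A single loop places each enemy at a random point inside the box, adjusting for collisions but always spawning.
; Spawning continues while the index is below one less than MaxEnemyNumbers; remaining iterations call CallSpawnFinished instead.
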(event `/Game/TDS/Blueprints/Spawner/BP_InterfaceSpawner.Spawn`
  (params (Player :type "TDSCharacter Object Reference"))
  (bind _maxenemynumbers (`self.MaxEnemyNumbers`))
  (for _index (range (+ _maxenemynumbers 1))
    (if (< _index (- _maxenemynumbers 1))
      (`|SpawnActorFromClass` (`self.EnemyClass`) (`KismetMathLibrary.Conv_VectorToTransform` (`KismetMathLibrary.RandomPointInBoundingBox` (`self.K2_GetActorLocation`) (`BoxComponent.GetScaledBoxExtent` (`self.Box`)))) "AdjustIfPossibleButAlwaysSpawn" "OverrideRootScale" null null)
      (else
        (`self.SpawnFinished`)))))

(fn `UserConstructionScript`)