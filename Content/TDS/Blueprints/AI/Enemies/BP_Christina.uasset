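; BP_Christina is a boss AI character in World 03 that also gates a door and can be flagged as talkable.
; Its death event forwards the bot name to the player controller's game widget to show Game Over.
; While it lives, player overlap with its sphere checks EnemyIsDead on the controller, then hides the mission border and calls OnShow.
; A valid Door then receives OpenDoorMessage, and the sphere destroys itself.
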(event `self.ReceiveBeginPlay`
  (add `self.OnBossDeath` (delegate `OnBossDeath_Event_0`)))

(event `OnBossDeath_Event_0` :!signature `self.OnBossDeath`
  (params (BotName :type Name))
  (bind _asbp_pc_03world (cast `/Game/TDS/Blueprints/Game/BP_PC_03World` (`GameplayStatics.GetPlayerController` 0)))
  (`/Engine/EditorBlueprintResources/StandardMacros.IsValid` _asbp_pc_03world
    (:`Is Valid`
      (bind _w_gamewidget (`/Game/TDS/Blueprints/Game/BP_PC_03World.W_GameWidget` _asbp_pc_03world))
      (`/Engine/EditorBlueprintResources/StandardMacros.IsValid` _w_gamewidget
        (:`Is Valid`
          (`/Game/TDS/UI/UI_03_Game/W_GameMain.OnShowGameOver` _w_gamewidget BotName))))))

(event `self.Sphere.OnComponentBeginOverlap`
  (params (OverlappedComponent :type "PrimitiveComponent Object Reference") (OtherActor :type "Actor Object Reference") (OtherComp :type "PrimitiveComponent Object Reference") (OtherBodyIndex :type Integer) (bFromSweep :type Boolean) (SweepResult :type "HitResult Structure (by ref)"))
  (bind _door (`self.Door`))
  (`/Engine/EditorBlueprintResources/StandardMacros.IsValid` self
    (:`Is Valid`
      (if (not (`TDSAIHealthComponent.IsDead` (`self.AIHealthComponent`)))
        (bind _asbp_player_character (cast `/Game/TDS/Blueprints/Character/BP_PlayerCharacter` OtherActor))
        (bind _asbp_pc_03world (cast `/Game/TDS/Blueprints/Game/BP_PC_03World` (`self.GetController` _asbp_player_character)))
        (if (`TDSPlayerController.EnemyIsDead` _asbp_pc_03world)
          (bind _output_get (set `self.As BP PC World` _asbp_pc_03world))
          (`/Engine/EditorBlueprintResources/StandardMacros.IsValid` _output_get
            (:`Is Valid`
              (bind _missionborder (`/Game/TDS/UI/UI_03_Game/W_GameMain.MissionBorder` (`/Game/TDS/Blueprints/Game/BP_PC_03World.W_GameWidget` _asbp_pc_03world)))
              (if (`Widget.IsVisible` _missionborder)
                (`Widget.SetVisibility` _missionborder "Hidden"))
              (`/Game/TDS/Blueprints/Game/BP_PC_03World.OnShow` _asbp_pc_03world)
              (`/Engine/EditorBlueprintResources/StandardMacros.IsValid` _door
                (:`Is Valid`
                  (message `/Game/TDS/Blueprints/Interfaces/BI_Collision.OpenDoor` _door)
                  (`ActorComponent.K2_DestroyComponent` (`self.Sphere`)))))))))))

(event `/Game/TDS/Blueprints/Interfaces/BI_Collision.TalkWithChristina`
  (set `self.IsCanTalk` true))

(fn `UserConstructionScript`)