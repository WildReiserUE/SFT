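; Player controller for a dialogue screen, likely for a dialogue map level, handling UI setup and keyboard navigation.
; On BeginPlay it shows the mouse cursor, creates the WBP_DialogueMap widget in the viewport and plays starter music.
; D/Right and A/Left call next and previous switching on WBPMainScreen unless its controls are disabled.
; The WBPMainScreen reference is not assigned in this graph and is separate from the created widget variable.
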(event `self.ReceiveBeginPlay`
  (set `self.bShowMouseCursor` true)
  (bind _returnvalue (`|CreateWidget` "/Game/TDS/UI/UI_02_Game/WBP_DialogueMap.WBP_DialogueMap_C" self))
  (`UserWidget.AddToViewport` _returnvalue 0)
  (`GameplayStatics.PlaySound2D` "/Game/TDS/Assets/Audio/Cue/Starter_Music_Cue.Starter_Music_Cue" 1.0 1.0 0.0 null null))

(event `Key|D`
  (params (Key :type "Key Structure"))
  (:`Pressed`
    (if (not (`/Game/TDS/UI/UI_02_Game/WBP_DialogueMap.bIsDisableControl` (`self.WBP_MainScreen`)))
      (`/Game/TDS/UI/UI_02_Game/WBP_DialogueMap.OnSwitchNext` (`self.WBP_MainScreen`)))))

(event `Key|Right`
  (params (Key :type "Key Structure"))
  (:`Pressed`
    (if (not (`/Game/TDS/UI/UI_02_Game/WBP_DialogueMap.bIsDisableControl` (`self.WBP_MainScreen`)))
      (`/Game/TDS/UI/UI_02_Game/WBP_DialogueMap.OnSwitchNext` (`self.WBP_MainScreen`)))))

(event `Key|A`
  (params (Key :type "Key Structure"))
  (bind _wbp_mainscreen (`self.WBP_MainScreen`))
  (:`Pressed`
    (if (not (`/Game/TDS/UI/UI_02_Game/WBP_DialogueMap.bIsDisableControl` _wbp_mainscreen))
      (`/Game/TDS/UI/UI_02_Game/WBP_DialogueMap.OnSwitchPrevious` _wbp_mainscreen))))

(event `Key|Left`
  (params (Key :type "Key Structure"))
  (bind _wbp_mainscreen (`self.WBP_MainScreen`))
  (:`Pressed`
    (if (not (`/Game/TDS/UI/UI_02_Game/WBP_DialogueMap.bIsDisableControl` _wbp_mainscreen))
      (`/Game/TDS/UI/UI_02_Game/WBP_DialogueMap.OnSwitchPrevious` _wbp_mainscreen))))

(fn `UserConstructionScript`)