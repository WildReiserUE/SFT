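; BP_CauserSpawn is a one-shot trigger actor that sets off linked spawners when a player character overlaps its collision component.
; On overlap it starts combat sound through the 03World game mode, then destroys itself immediately if the player is on Team1.
; For other teams it first calls OnShow on the player controller if the game widget's row sequence matches Current, and sends SpawnMessage to each referenced spawner.
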(event `self.CollisionComponent.OnComponentBeginOverlap`
  (params (OverlappedComponent :type "PrimitiveComponent Object Reference") (OtherActor :type "Actor Object Reference") (OtherComp :type "PrimitiveComponent Object Reference") (OtherBodyIndex :type Integer) (bFromSweep :type Boolean) (SweepResult :type "HitResult Structure (by ref)"))
  (bind _spawners (`self.Spawners`))
  (bind _asbp_player_character (cast `/Game/TDS/Blueprints/Character/BP_PlayerCharacter` OtherActor))
  (bind _asbp_gm_03world (cast `/Game/TDS/Blueprints/Game/BP_GM_03World` (`GameplayStatics.GetGameMode`)))
  (`/Game/TDS/Blueprints/Game/BP_GM_03World.StartSoundCombat` _asbp_gm_03world)
  (if (`|EnumEquality` (`TDSCharacter.NewTeamID` _asbp_player_character) "Team_1")
    (`self.K2_DestroyActor`)
    (else
      (`self.TryToShowWidget` _asbp_player_character)
      (for (_array_element _array_index) _spawners
        (if (`KismetArrayLibrary.Array_IsValidIndex` _spawners _array_index)
          (message `/Game/TDS/Blueprints/Spawner/BP_InterfaceSpawner.Spawn` _array_element _asbp_player_character)))
      (`self.K2_DestroyActor`))))

(fn `TryToShowWidget`
  (params (self2 :type "Actor Object Reference"))
  (bind _asbp_pc_03world (cast `/Game/TDS/Blueprints/Game/BP_PC_03World` (`Pawn.GetController` (`Actor.Instigator` self2))))
  (if (== (`/Game/TDS/UI/UI_03_Game/W_GameMain.Row Sequence` (`/Game/TDS/Blueprints/Game/BP_PC_03World.W_GameWidget` _asbp_pc_03world)) (`self.Current`))
    (`/Game/TDS/Blueprints/Game/BP_PC_03World.OnShow` _asbp_pc_03world)))

(fn `UserConstructionScript`)