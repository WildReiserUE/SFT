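; BP_DoorSecondFloor is a door that opens for the player only when the BP_PC_03World controller reports the enemy is dead.
; A Check function gates the Box overlap events by casting to BP_PlayerCharacter and its controller, then querying EnemyIsDead.
; Entering plays a timeline that slides DoorMesh down along relative Z, and leaving reverses it after a short delay.
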(event `self.Box.OnComponentBeginOverlap`
  (params (OverlappedComponent :type "PrimitiveComponent Object Reference") (OtherActor :type "Actor Object Reference") (OtherComp :type "PrimitiveComponent Object Reference") (OtherBodyIndex :type Integer) (bFromSweep :type Boolean) (SweepResult :type "HitResult Structure (by ref)"))
  (bind _isopendoor (`self.Check` OtherActor))
  (if _isopendoor
    (bind (_direction _newtrack_0) (`Timeline|Timeline_1` :!label _label)
      (:`Update`
        (`SceneComponent.K2_SetRelativeLocation` (`self.DoorMesh`) (`KismetMathLibrary.MakeVector` 0.0 0.0 (`KismetMathLibrary.Lerp` 0.0 -25.0 _newtrack_0)) false false)))))

(event `self.Box.OnComponentEndOverlap`
  (params (OverlappedComponent :type "PrimitiveComponent Object Reference") (OtherActor :type "Actor Object Reference") (OtherComp :type "PrimitiveComponent Object Reference") (OtherBodyIndex :type Integer))
  (bind _isopendoor (`self.Check` OtherActor))
  (if _isopendoor
    (`KismetSystemLibrary.Delay` 1.5)
    (goto _label :!via `Reverse`)))

(fn `Check`
  (params (Object :type "Object Object Reference"))
  (returns (IsOpenDoor :type Boolean))
  (bind _asbp_player_character (cast `/Game/TDS/Blueprints/Character/BP_PlayerCharacter` Object))
  (bind _asbp_pc_03world (cast `/Game/TDS/Blueprints/Game/BP_PC_03World` (`Pawn.GetController` _asbp_player_character)))
  (if (`TDSPlayerController.EnemyIsDead` _asbp_pc_03world)
    (return true)
    (else
      (return false))))

(fn `UserConstructionScript`)