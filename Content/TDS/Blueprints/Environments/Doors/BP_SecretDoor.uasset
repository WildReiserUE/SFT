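; BP_SecretDoor is a secret door that opens when the player character enters its trigger box carrying the required item.
; On overlap it searches the player's inventory for IDItemToOpen and, if found, sets IsOpen and plays a timeline that lerps the door mesh downward.
; The door stays open, as end overlap does nothing and the reverse-timeline closing logic is left disconnected.
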(event `self.Box.OnComponentBeginOverlap`
  (params (OverlappedComponent :type "PrimitiveComponent Object Reference") (OtherActor :type "Actor Object Reference") (OtherComp :type "PrimitiveComponent Object Reference") (OtherBodyIndex :type Integer) (bFromSweep :type Boolean) (SweepResult :type "HitResult Structure (by ref)"))
  (if (not (`self.bIsOpen?`))
    (bind _asbp_player_character (cast `/Game/TDS/Blueprints/Character/BP_PlayerCharacter` OtherActor))
    (bind _returnvalue (`TDSInventoryComponent.FindItemById` (`TDSCharacter.PlayerInventory` _asbp_player_character) (`self.ID_Item-To_Open`)))
    (if (> _returnvalue -1)
      (set `self.bIsOpen?` true)
      (bind (_direction _newtrack_0) (`Timeline|Timeline_0`)
        (:`Update`
          (`SceneComponent.K2_SetRelativeLocation` (`self.Door`) (`KismetMathLibrary.MakeVector` 0.0 0.0 (`KismetMathLibrary.Lerp` 0.0 -30.0 _newtrack_0)) false false))))))

(event `self.Box.OnComponentEndOverlap`
  (params (OverlappedComponent :type "PrimitiveComponent Object Reference") (OtherActor :type "Actor Object Reference") (OtherComp :type "PrimitiveComponent Object Reference") (OtherBodyIndex :type Integer)))

(fn `UserConstructionScript`)