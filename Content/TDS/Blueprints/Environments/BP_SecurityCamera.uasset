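; BP_SecurityCamera is a sweeping security camera that flags when the player is inside its view cone.
; Each tick the lens mesh yaws by Delta, and a looping timer flips the sign of Delta to sweep it back and forth.
; Overlap events on the view cone mesh set a Material Parameter Collection scalar on and off as BP_PlayerCharacter enters and leaves.
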(event `self.ReceiveBeginPlay`
  (`KismetSystemLibrary.K2_SetTimerDelegate` (delegate `ChangeDirection`) 6.0 true))

(event `ChangeDirection`
  (set `self.Delta` (* -1 (`self.Delta`))))

(event `self.ReceiveTick`
  (params (DeltaSeconds :type "Float (single-precision)"))
  (`SceneComponent.K2_AddLocalRotation` (`self.SM_Security_Camera_Lens`) (`KismetMathLibrary.MakeRotator` 0.0 0.0 (`self.Delta`)) false false))

(event `self.SM_Security_Camera_Viewcone.OnComponentBeginOverlap`
  (params (OverlappedComponent :type "PrimitiveComponent Object Reference") (OtherActor :type "Actor Object Reference") (OtherComp :type "PrimitiveComponent Object Reference") (OtherBodyIndex :type Integer) (bFromSweep :type Boolean) (SweepResult :type "HitResult Structure (by ref)"))
  (cast `/Game/TDS/Blueprints/Character/BP_PlayerCharacter` OtherActor)
  (`KismetMaterialLibrary.SetScalarParameterValue` (`self.MaterialParametr`) (`self.Parameter Name`) 1.0))

(event `self.SM_Security_Camera_Viewcone.OnComponentEndOverlap`
  (params (OverlappedComponent :type "PrimitiveComponent Object Reference") (OtherActor :type "Actor Object Reference") (OtherComp :type "PrimitiveComponent Object Reference") (OtherBodyIndex :type Integer))
  (cast `/Game/TDS/Blueprints/Character/BP_PlayerCharacter` OtherActor)
  (`KismetMaterialLibrary.SetScalarParameterValue` (`self.MaterialParametr`) (`self.Parameter Name`) 0.0))

(fn `UserConstructionScript`)