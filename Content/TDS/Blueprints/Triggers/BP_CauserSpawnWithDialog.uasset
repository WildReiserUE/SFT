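; One-shot trigger volume that, on player overlap, disables its collision, starts combat sound through BP_GM_03World and begins a looping spawn timer.
; Each tick plays a sound, calls SpawnMessage on a random Spawners entry and removes one, re-rolling the index each time, so they can differ.
; The timer clears and the actor destroys itself only if removal fails.
; TryToShowWidget only casts the player controller, showing nothing.
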(event `self.CollisionComponent.OnComponentBeginOverlap`
  (params (OverlappedComponent :type "PrimitiveComponent Object Reference") (OtherActor :type "Actor Object Reference") (OtherComp :type "PrimitiveComponent Object Reference") (OtherBodyIndex :type Integer) (bFromSweep :type Boolean) (SweepResult :type "HitResult Structure (by ref)"))
  (bind _asbp_player_character (cast `/Game/TDS/Blueprints/Character/BP_PlayerCharacter` OtherActor))
  (`PrimitiveComponent.SetCollisionResponseToAllChannels` (`self.CollisionComponent`) "ECR_Ignore")
  (bind _asbp_gm_03world (cast `/Game/TDS/Blueprints/Game/BP_GM_03World` (`GameplayStatics.GetGameMode`)))
  (`/Game/TDS/Blueprints/Game/BP_GM_03World.StartSoundCombat` _asbp_gm_03world)
  (`self.TryToShowWidget` _asbp_player_character)
  (bind _returnvalue (`KismetSystemLibrary.K2_SetTimerDelegate` (delegate `StartSpawn`) 0.5 true))
  (set `self.HTimer` _returnvalue))

(event `StartSpawn`
  (bind _spawners (`self.Spawners`))
  (bind _returnvalue (`KismetMathLibrary.RandomIntegerInRange` 0 (`KismetArrayLibrary.Array_LastIndex` _spawners)))
  (bind _output (`|GetArrayItem` _spawners _returnvalue))
  (if (> (`KismetArrayLibrary.Array_Length` _spawners) 0)
    (if (`KismetArrayLibrary.Array_IsValidIndex` _spawners _returnvalue)
      (`GameplayStatics.PlaySound2D` (`self.SpawnSound`) 1.0 1.0 0.0 null null)
      (message `/Game/TDS/Blueprints/Spawner/BP_InterfaceSpawner.Spawn` _output (stale `self.CollisionComponent.OnComponentBeginOverlap` _asbp_player_character))
      (bind _returnvalue_2 (`KismetArrayLibrary.Array_RemoveItem` _spawners _output))
      (if (not _returnvalue_2)
        (`KismetSystemLibrary.K2_ClearAndInvalidateTimerHandle` (`self.HTimer`))
        (`self.K2_DestroyActor`)))))

(fn `TryToShowWidget`
  (params (self2 :type "Actor Object Reference"))
  (cast `/Game/TDS/Blueprints/Game/BP_PC_03World` (`Pawn.GetController` (`Actor.Instigator` self2))))

(fn `UserConstructionScript`)