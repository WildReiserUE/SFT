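; BP_Elevator is an elevator actor that travels vertically when the player character steps into its trigger.
; The first overlap waits briefly, records the current height, then plays the ZMove timeline to offset the actor's Z from it.
; A DoorStartClose event from the referenced WhatStateDoor clears the position flag and reverses the timeline to send the elevator back.
; A moving sound plays during travel and an end sound when the timeline finishes.
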(event `self.TriggerContact.OnComponentBeginOverlap`
  (params (OverlappedComponent :type "PrimitiveComponent Object Reference") (OtherActor :type "Actor Object Reference") (OtherComp :type "PrimitiveComponent Object Reference") (OtherBodyIndex :type Integer) (bFromSweep :type Boolean) (SweepResult :type "HitResult Structure (by ref)"))
  (bind (_returnvalue_x _returnvalue_y _returnvalue_z) (`KismetMathLibrary.BreakVector` (`self.K2_GetActorLocation`)))
  (cast `/Game/TDS/Blueprints/Character/BP_PlayerCharacter` OtherActor)
  (if (not (`self.bIsStartPos?`))
    (set `self.bIsStartPos?` true)
    (`KismetSystemLibrary.Delay` 0.5)
    (`AudioComponent.Play` (`self.AudioMoving`) 0.0)
    (set `self.LocZToStart` _returnvalue_z)
    (bind (_direction _z) (`Timeline|Z-Move` :!via `PlayFromStart` :!label _label)
      (:`Update`
        (`self.K2_SetActorLocation` (`KismetMathLibrary.MakeVector` _returnvalue_x _returnvalue_y (+ (`self.LocZToStart`) _z))))
      (:`Finished`
        (`AudioComponent.Stop` (`self.AudioMoving`))
        (`AudioComponent.Play` (`self.AudioEndMove`) 0.0)))))

(event `self.WhatStateDoor.DoorStartClose`
  (`AudioComponent.Play` (`self.AudioMoving`) 0.0)
  (set `self.bIsStartPos?` false)
  (goto _label :!via `Reverse`))

(fn `UserConstructionScript`)