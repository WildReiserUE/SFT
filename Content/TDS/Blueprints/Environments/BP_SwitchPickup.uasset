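; BP_SwitchPickup is an interactable switch pickup with a custom-depth mesh highlight, whose interaction so far only prints a debug message.
; BeginPlay enables custom depth on the mesh, and sphere overlaps with BP_PlayerCharacter toggle IsCanClick and the sphere component's own visibility.
; Pressing E while IsCanClick is true turns off the mesh's custom depth, hides the text render and prints "Hello".
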(event `self.ReceiveBeginPlay`
  (`PrimitiveComponent.SetRenderCustomDepth` (`self.StaticMesh`) true))

(event `Key|E`
  (params (Key :type "Key Structure"))
  (:`Pressed`
    (if (`self.IsCanClick`)
      (`PrimitiveComponent.SetRenderCustomDepth` (`self.StaticMesh`) false)
      (`SceneComponent.SetVisibility` (`self.TextRender`) false false)
      (`KismetSystemLibrary.PrintString` "Hello"))))

(event `self.SphereComponent.OnComponentBeginOverlap`
  (params (OverlappedComponent :type "PrimitiveComponent Object Reference") (OtherActor :type "Actor Object Reference") (OtherComp :type "PrimitiveComponent Object Reference") (OtherBodyIndex :type Integer) (bFromSweep :type Boolean) (SweepResult :type "HitResult Structure (by ref)"))
  (cast `/Game/TDS/Blueprints/Character/BP_PlayerCharacter` OtherActor)
  (set `self.IsCanClick` true)
  (`SceneComponent.SetVisibility` (`self.SphereComponent`) true false))

(event `self.SphereComponent.OnComponentEndOverlap`
  (params (OverlappedComponent :type "PrimitiveComponent Object Reference") (OtherActor :type "Actor Object Reference") (OtherComp :type "PrimitiveComponent Object Reference") (OtherBodyIndex :type Integer))
  (cast `/Game/TDS/Blueprints/Character/BP_PlayerCharacter` OtherActor)
  (set `self.IsCanClick` false)
  (`SceneComponent.SetVisibility` (`self.SphereComponent`) false false))

(fn `UserConstructionScript`)