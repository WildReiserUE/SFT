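; BP_GasCamera is a temporary gas effect actor that plays audio, rapidly expands, lingers, then shrinks away and destroys itself.
; BeginPlay seeds StartScale from the PSteamLit component's world scale and starts a fast looping timer that multiplies the whole actor's scale up to a cap.
; After a short delay, a second looping timer shrinks it geometrically until the minimum threshold triggers destruction.
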(event `self.ReceiveBeginPlay`
  (set `self.StartScale` (`SceneComponent.K2_GetComponentScale` (`self.P_Steam_Lit`)))
  (bind _returnvalue (`KismetSystemLibrary.K2_SetTimerDelegate` (delegate `Scale`) 0.01 true))
  (set `self.Timer` _returnvalue)
  (`AudioComponent.Play` (`self.Audio`) 0.0))

(event `Scale`
  (bind (_returnvalue_location _returnvalue_rotation) (`KismetMathLibrary.BreakTransform` (`self.GetTransform`)))
  (bind (_startscale_x _startscale_y _startscale_z) (`KismetMathLibrary.BreakVector` (`self.StartScale`)))
  (bind _returnvalue (* _startscale_x 10.0))
  (if (>= _returnvalue 1000.0)
    (`KismetSystemLibrary.K2_ClearAndInvalidateTimerHandle` (`self.Timer`))
    (`KismetSystemLibrary.Delay` 5.0)
    (bind _returnvalue_2 (`KismetSystemLibrary.K2_SetTimerDelegate` (delegate `Smaller`) 0.01 true))
    (set `self.Timer2` _returnvalue_2)
    (else
      (bind _output_get (set `self.StartScale` (`KismetMathLibrary.MakeVector` _returnvalue (* _startscale_y 10.0) (* _startscale_z 10.0))))
      (`self.K2_SetActorTransform` (`KismetMathLibrary.MakeTransform` _returnvalue_location _returnvalue_rotation (`KismetMathLibrary.MakeVector` (.x _output_get) (.y _output_get) (.z _output_get)))))))

(event `Smaller`
  (bind (_returnvalue_location _returnvalue_rotation) (`KismetMathLibrary.BreakTransform` (`self.GetTransform`)))
  (bind (_startscale_x _startscale_y _startscale_z) (`KismetMathLibrary.BreakVector` (`self.StartScale`)))
  (bind _returnvalue (* _startscale_x 0.9))
  (if (<= _returnvalue 0.01)
    (`KismetSystemLibrary.K2_ClearAndInvalidateTimerHandle` (`self.Timer2`))
    (`self.K2_DestroyActor`)
    (else
      (bind _output_get (set `self.StartScale` (`KismetMathLibrary.MakeVector` _returnvalue (* _startscale_y 0.9) (* _startscale_z 0.9))))
      (`self.K2_SetActorTransform` (`KismetMathLibrary.MakeTransform` _returnvalue_location _returnvalue_rotation (`KismetMathLibrary.MakeVector` (.x _output_get) (.y _output_get) (.z _output_get)))))))

(fn `UserConstructionScript`)