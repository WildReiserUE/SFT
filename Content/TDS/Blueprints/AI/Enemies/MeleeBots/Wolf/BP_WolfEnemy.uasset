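; BP_WolfEnemy is a Wolf melee bot enemy whose boss death ends play in the 03World level.
; On BeginPlay it binds to its boss death event, which pauses the game and reveals the final game screen in the player controller's HUD widget.
; Tick, overlap and construction are empty, and a leftover health-component death check is never executed.
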(event `self.ReceiveBeginPlay`
  (add `self.OnBossDeath` (delegate `OnBossDeath_Event_0`)))

(event `OnBossDeath_Event_0` :!signature `self.OnBossDeath`
  (params (BotName :type Name))
  (bind _asbp_pc_03world (cast `/Game/TDS/Blueprints/Game/BP_PC_03World` (`GameplayStatics.GetPlayerController` 0)))
  (`/Engine/EditorBlueprintResources/StandardMacros.IsValid` _asbp_pc_03world
    (:`Is Valid`
      (`GameplayStatics.SetGamePaused` true)
      (`Widget.SetVisibility` (`/Game/TDS/UI/UI_03_Game/W_GameMain.WBP_GameFinal` (`/Game/TDS/Blueprints/Game/BP_PC_03World.W_GameWidget` _asbp_pc_03world)) "Visible"))))

(event `self.ReceiveTick`
  (params (DeltaSeconds :type "Float (single-precision)")))

(fn `UserConstructionScript`)