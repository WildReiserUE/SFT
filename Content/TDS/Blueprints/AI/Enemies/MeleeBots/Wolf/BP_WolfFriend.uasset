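; BP_WolfFriend is a wolf actor that triggers a dialog when the player approaches it.
; On sphere overlap it casts to BP_PlayerCharacter and gets its BP_PC_03World controller.
; If the controller reports the enemy dead and its game widget's Index matches a hard-coded step, it calls OnShowDialog on that widget.
; Debug prints report which check passed or failed, while BeginPlay, Tick and construction are empty.
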(event `self.ReceiveBeginPlay`)

(event `self.ReceiveTick`
  (params (DeltaSeconds :type "Float (single-precision)")))

(event `self.Sphere.OnComponentBeginOverlap`
  (params (OverlappedComponent :type "PrimitiveComponent Object Reference") (OtherActor :type "Actor Object Reference") (OtherComp :type "PrimitiveComponent Object Reference") (OtherBodyIndex :type Integer) (bFromSweep :type Boolean) (SweepResult :type "HitResult Structure (by ref)"))
  (bind _asbp_player_character (cast `/Game/TDS/Blueprints/Character/BP_PlayerCharacter` OtherActor))
  (`/Engine/EditorBlueprintResources/StandardMacros.IsValid` _asbp_player_character
    (:`Is Valid`
      (bind _asbp_pc_03world (cast `/Game/TDS/Blueprints/Game/BP_PC_03World` (`self.GetController` _asbp_player_character)))
      (if (`TDSPlayerController.EnemyIsDead` _asbp_pc_03world)
        (`KismetSystemLibrary.PrintString` "Success_1")
        (bind _w_gamewidget (`/Game/TDS/Blueprints/Game/BP_PC_03World.W_GameWidget` _asbp_pc_03world))
        (bind _index (`/Game/TDS/UI/UI_03_Game/W_GameMain.Index` _w_gamewidget))
        (if (== _index 20)
          (`KismetSystemLibrary.PrintString` "Success_2")
          (`/Game/TDS/UI/UI_03_Game/W_GameMain.OnShowDialog` _w_gamewidget)
          (else
            (`KismetSystemLibrary.PrintString` (`KismetStringLibrary.Conv_IntToString` _index))))
        (else
          (`KismetSystemLibrary.PrintString` "Failed_1"))))))

(fn `UserConstructionScript`)