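; Game mode for the 03 World level that handles staged player spawning and switches music between search and combat.
; Players start at the Stage1 start; respawning asks BP_GS_World for permission and uses the current stage's named start.
; A spawned AmbientSound plays the music, with EndSound fading combat out by looping timer before restoring the search track.
; Separate countdown-based fade helpers exist but are not wired into these events.
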(event `self.ReceiveBeginPlay`
  (set `self.Timer` (`self.MaxTimer`))
  (bind _returnvalue (`|SpawnActorFromClass` "/Script/Engine.AmbientSound" (`KismetMathLibrary.MakeTransform` (0.0 0.0 0.0)) "Undefined" "OverrideRootScale" null null))
  (bind _output_get (set `self.LevelSound` _returnvalue))
  (`/Engine/EditorBlueprintResources/StandardMacros.IsValid` _output_get
    (:`Is Valid`
      (bind _audiocomponent (`AmbientSound.AudioComponent` _output_get))
      (`AudioComponent.SetSound` _audiocomponent "/Game/TDS/Assets/Audio/Cue/Mixdown_Cue.Mixdown_Cue")
      (`AudioComponent.Play` _audiocomponent 0.0))))

(event `StartSoundCombat`
  (bind _audiocomponent (`AmbientSound.AudioComponent` (`self.LevelSound`)))
  (`AudioComponent.SetSound` _audiocomponent "/Game/TDS/Assets/Audio/Cue/A_Bear_From_Outer_Space_Cue.A_Bear_From_Outer_Space_Cue")
  (`AudioComponent.SetVolumeMultiplier` _audiocomponent 0.5)
  (`AudioComponent.Play` _audiocomponent 0.0))

(event `EndSound`
  (bind _audiocomponent (`AmbientSound.AudioComponent` (`self.LevelSound`)))
  (bind _volumemultiplier (`AudioComponent.VolumeMultiplier` _audiocomponent))
  (bind _returnvalue (`KismetSystemLibrary.K2_SetTimerDelegate` (delegate `EndSound`) 0.5 true))
  (if (> _volumemultiplier 0.0)
    (`AudioComponent.SetVolumeMultiplier` _audiocomponent (- _volumemultiplier 0.1))
    (else
      (`KismetSystemLibrary.K2_ClearAndInvalidateTimerHandle` _returnvalue)
      (`self.StartSoundSearch`))))

(event `StartSoundSearch`
  (bind _audiocomponent (`AmbientSound.AudioComponent` (`self.LevelSound`)))
  (`AudioComponent.SetSound` _audiocomponent "/Game/TDS/Assets/Audio/Cue/Mixdown_Cue.Mixdown_Cue")
  (`AudioComponent.SetVolumeMultiplier` _audiocomponent 0.9)
  (`AudioComponent.Play` _audiocomponent 0.0))

(fn `ChoosePlayerStart`
  (params (Player :type "Controller Object Reference"))
  (returns (ReturnValue :type "Actor Object Reference"))
  (return (`self.K2_FindPlayerStart` Player "Stage1")))

(fn `Play`
  (params (self2 :type "AudioComponent Object Reference"))
  (`AudioComponent.Play` self2 0.0)
  (`self.StartSound` (struct)))

(fn `StartSound`
  (params (NewParam :type "TimerHandle Structure"))
  (bind _audiocomponent (`AmbientSound.AudioComponent` (`self.LevelSound`)))
  (bind _output_get (set `self.Timer` (- (`self.Timer`) 1)))
  (if (or (<= (`AudioComponent.VolumeMultiplier` (`AmbientSound.AudioComponent` (`self.LevelSound`))) 0.5) (> _output_get 0))
    (`AudioComponent.SetVolumeMultiplier` _audiocomponent (+ (`AudioComponent.VolumeMultiplier` _audiocomponent) 0.1))
    (else
      (`KismetSystemLibrary.K2_ClearAndInvalidateTimerHandle` NewParam)
      (set `self.Timer` (`self.MaxTimer`)))))

(fn `Stop`
  (params (Handle :type "TimerHandle Structure (by ref)"))
  (returns (IsCanChangeSound :type Boolean))
  (bind _audiocomponent (`AmbientSound.AudioComponent` (`self.LevelSound`)))
  (set `self.Timer` (- (`self.Timer`) 1))
  (if (or (> (`AudioComponent.VolumeMultiplier` (`AmbientSound.AudioComponent` (`self.LevelSound`))) 0.0) (> (`self.Timer`) 0))
    (`AudioComponent.SetVolumeMultiplier` _audiocomponent (- (`AudioComponent.VolumeMultiplier` _audiocomponent) 0.1))
    (else
      (`KismetSystemLibrary.K2_ClearAndInvalidateTimerHandle` Handle)
      (`AudioComponent.Stop` (`AmbientSound.AudioComponent` (`self.LevelSound`)))
      (set `self.Timer` (`self.MaxTimer`))
      (return true))))

(fn `TryToRespawn`
  (returns (Success :type Boolean))
  (bind _returnvalue (`GameplayStatics.GetPlayerController` 0))
  (bind _asbp_gs_world (cast `/Game/TDS/Blueprints/Game/BP_GS_World` (`GameplayStatics.GetGameState`)))
  (bind (_bissuccess _e_currentstage) (`/Game/TDS/Blueprints/Game/BP_GS_World.CanPlayerRespawn` _asbp_gs_world))
  (if _bissuccess
    (`self.RestartPlayerAtPlayerStart` _returnvalue (`self.K2_FindPlayerStart` _returnvalue (select `/Game/TDS/Blueprints/Game/E_LevelStage` _e_currentstage :`NewEnumerator0` "Stage1" :`NewEnumerator1` "Stage2" :`NewEnumerator2` "Stage3" :`NewEnumerator3` "Stage4")))
    (return _bissuccess)
    (else
      (return _bissuccess))))

(fn `UserConstructionScript`)