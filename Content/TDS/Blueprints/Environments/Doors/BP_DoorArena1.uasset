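; Arena door actor that opens and closes along Z as the player character passes through its trigger boxes.
; BoxIN starts a short delay, then plays a sound and a timeline offsetting the door from its saved height.
; BoxOUT reverses that timeline with sound and calls DoorStartClose.
; A state flag gates each direction; triggers ignore collision once hit and both re-enable when the timeline finishes.
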(event `self.BoxIN.OnComponentBeginOverlap`
  (params (OverlappedComponent :type "PrimitiveComponent Object Reference") (OtherActor :type "Actor Object Reference") (OtherComp :type "PrimitiveComponent Object Reference") (OtherBodyIndex :type Integer) (bFromSweep :type Boolean) (SweepResult :type "HitResult Structure (by ref)"))
  (bind (_returnvalue_x _returnvalue_y _returnvalue_z) (`KismetMathLibrary.BreakVector` (`self.K2_GetActorLocation`)))
  (cast `/Game/TDS/Blueprints/Character/BP_PlayerCharacter` OtherActor)
  (`PrimitiveComponent.SetCollisionResponseToAllChannels` (`self.BoxIN`) "ECR_Ignore")
  (if (not (`self.bIsStartPos?`))
    (set `self.bIsStartPos?` true)
    (`KismetSystemLibrary.Delay` 0.5)
    (`AudioComponent.Play` (`self.MoveSound`) 0.0)
    (set `self.LocZToStart` _returnvalue_z)
    (bind (_direction _z) (`Timeline|Timeline_0` :!via `PlayFromStart` :!label _label)
      (:`Update`
        (`self.K2_SetActorLocation` (`KismetMathLibrary.MakeVector` _returnvalue_x _returnvalue_y (+ (`self.LocZToStart`) _z))))
      (:`Finished`
        (`PrimitiveComponent.SetCollisionResponseToAllChannels` (`self.BoxIN`) "ECR_Overlap")
        (`PrimitiveComponent.SetCollisionResponseToAllChannels` (`self.BoxOUT`) "ECR_Overlap")))))

(event `self.BoxOUT.OnComponentBeginOverlap`
  (params (OverlappedComponent :type "PrimitiveComponent Object Reference") (OtherActor :type "Actor Object Reference") (OtherComp :type "PrimitiveComponent Object Reference") (OtherBodyIndex :type Integer) (bFromSweep :type Boolean) (SweepResult :type "HitResult Structure (by ref)"))
  (cast `/Game/TDS/Blueprints/Character/BP_PlayerCharacter` OtherActor)
  (`PrimitiveComponent.SetCollisionResponseToAllChannels` (`self.BoxOUT`) "ECR_Ignore")
  (if (`self.bIsStartPos?`)
    (set `self.bIsStartPos?` false)
    (`AudioComponent.Play` (`self.MoveSound`) 0.0)
    (`self.DoorStartClose`)
    (goto _label :!via `Reverse`)))

(fn `UserConstructionScript`)