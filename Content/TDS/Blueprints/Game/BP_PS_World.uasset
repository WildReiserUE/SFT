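; BP_PS_World is a TDS Blueprint, apparently a PlayerState, that holds saved copies of the player's weapon set and diary.
; SaveCurrentWeapon and SaveCurrentDiary each resize the stored array to match the input, then copy it element by element.
; GetSavedWeapon returns the stored weapon set, while the diary has no getter here.
; BeginPlay only calls the parent, and nothing in this Blueprint writes to disk.
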(event `self.ReceiveBeginPlay`
  (`parent.ReceiveBeginPlay`))

(fn `GetSavedWeapon`
  (returns (SavedStruct :type "Array of TDSWeaponBase Class Reference"))
  (return (`self.SavedWeapon Set`)))

(fn `SaveCurrentDiary`
  (params (TDSDiary :type "Array of TDSDiary Class Reference"))
  (bind _savestdsdiary (`self.SavesTDSDiary`))
  (`KismetArrayLibrary.Array_Resize` _savestdsdiary (`KismetArrayLibrary.Array_Length` TDSDiary))
  (for (_array_element _array_index) TDSDiary
    (`KismetArrayLibrary.Array_Set` _savestdsdiary _array_index _array_element)))

(fn `SaveCurrentWeapon`
  (params (WeaponSet :type "Array of TDSWeaponBase Class Reference"))
  (bind _savedweapon_set (`self.SavedWeapon Set`))
  (`KismetArrayLibrary.Array_Resize` _savedweapon_set (`KismetArrayLibrary.Array_Length` WeaponSet))
  (for (_array_element _array_index) WeaponSet
    (`KismetArrayLibrary.Array_Set` _savedweapon_set _array_index _array_element)))

(fn `UserConstructionScript`)