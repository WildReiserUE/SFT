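; Arena door actor that lowers when the player enters one of its two trigger boxes and the World 03 player controller reports the enemy dead.
; Both BoxIN and BoxOUT overlaps share one path that plays a sound, stores the current Z and runs a timeline subtracting from it.
; OpenDoor only prints a debug string, and a mission-close widget call is left unconnected.
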(event `self.BoxIN.OnComponentBeginOverlap`
  (params (OverlappedComponent :type "PrimitiveComponent Object Reference") (OtherActor :type "Actor Object Reference") (OtherComp :type "PrimitiveComponent Object Reference") (OtherBodyIndex :type Integer) (bFromSweep :type Boolean) (SweepResult :type "HitResult Structure (by ref)"))
  (bind (_returnvalue_x _returnvalue_y _returnvalue_z) (`KismetMathLibrary.BreakVector` (`self.K2_GetActorLocation`)))
  (bind _asbp_player_character (cast `/Game/TDS/Blueprints/Character/BP_PlayerCharacter` OtherActor))
  (bind _asbp_pc_03world (cast `/Game/TDS/Blueprints/Game/BP_PC_03World` (`Pawn.GetController` _asbp_player_character)))
  (if (`TDSPlayerController.EnemyIsDead` _asbp_pc_03world)
    (`AudioComponent.Play` (`self.MoveSound`) 0.0 :!label _label)
    (set `self.LocZToStart` _returnvalue_z)
    (bind (_direction _z) (`Timeline|Timeline_0`)
      (:`Update`
        (`self.K2_SetActorLocation` (`KismetMathLibrary.MakeVector` _returnvalue_x _returnvalue_y (- (`self.LocZToStart`) _z)))))))

(event `self.BoxOUT.OnComponentBeginOverlap`
  (params (OverlappedComponent :type "PrimitiveComponent Object Reference") (OtherActor :type "Actor Object Reference") (OtherComp :type "PrimitiveComponent Object Reference") (OtherBodyIndex :type Integer) (bFromSweep :type Boolean) (SweepResult :type "HitResult Structure (by ref)"))
  (bind _asbp_player_character (cast `/Game/TDS/Blueprints/Character/BP_PlayerCharacter` OtherActor))
  (bind _asbp_pc_03world (cast `/Game/TDS/Blueprints/Game/BP_PC_03World` (`Pawn.GetController` _asbp_player_character)))
  (if (`TDSPlayerController.EnemyIsDead` _asbp_pc_03world)
    (goto _label)))

(event `/Game/TDS/Blueprints/Interfaces/BI_Collision.OpenDoor`
  (`KismetSystemLibrary.PrintString` "Hello"))

(fn `UserConstructionScript`)