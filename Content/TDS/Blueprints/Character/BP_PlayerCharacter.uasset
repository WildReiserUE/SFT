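; BP_PlayerCharacter is the player-controlled character for the TDS game, handling damage feedback, death and camera setup.
; Health changes play a hit sound with random blood decals, or on death save weapons and diary to BP_PS_World, disable collision and play a montage.
; Receiving an inventory item can close the mission widget through BP_PC_03World, and F plays a twist animation.
; The construction script applies exposed camera arm length, lag and rotation settings.
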(event `self.ReceiveBeginPlay`
  (`PrimitiveComponent.SetCollisionEnabled` (`self.CapsuleComponent`) "QueryAndPhysics")
  (add `TDSInventoryComponent.OnReceiveItem` (`self.PlayerInventory`) (delegate `OnReceiveItem_Event_0`)))

(event `OnReceiveItem_Event_0`
  (if (`self.ShowMission`)
    (bind _asbp_pc_03world (cast `/Game/TDS/Blueprints/Game/BP_PC_03World` (`self.GetController`)))
    (`/Engine/EditorBlueprintResources/StandardMacros.IsValid` _asbp_pc_03world
      (:`Is Valid`
        (if (`/Game/TDS/Blueprints/Game/BP_PC_03World.bIsShowJuice` _asbp_pc_03world)
          (`/Game/TDS/UI/UI_03_Game/W_GameMain.OnCloseMission` (`/Game/TDS/Blueprints/Game/BP_PC_03World.W_GameWidget` _asbp_pc_03world))
          (set `self.ShowMission` false))))))

(event `self.PlayerStateInfo.OnHealthChange`
  (params (Health :type "Float (single-precision)") (MaxHealthValue :type "Float (single-precision)"))
  (if (<= Health 0.0)
    (`KismetSystemLibrary.Delay` 0.1)
    (`self.SaveInventory` (`GameplayStatics.GetPlayerController` 0))
    (`PrimitiveComponent.SetCollisionEnabled` (`self.CapsuleComponent`) "NoCollision")
    (`PrimitiveComponent.SetCollisionEnabled` (`self.Mesh`) "NoCollision")
    (`|PlayMontage` (`self.Mesh`) "/Game/TDS/Assets/Player/Mihail/AM_Mihael_Death1.AM_Mihael_Death1")
    (elif (> Health 0.0)
      (`GameplayStatics.PlaySound2D` "/Game/TDS/Assets/Audio/Cue/Hit_Receive.Hit_Receive" 1.0 1.0 0.0 null null)
      (if (>= (`KismetMathLibrary.RandomFloatInRange` 0.0 10.0) 2.0)
        (`GameplayStatics.SpawnDecalAtLocation` (`self.BloodDecal`) (30.0 120.0 120.0) (- (`self.K2_GetActorLocation`) (`KismetMathLibrary.MakeVector` (`KismetMathLibrary.RandomFloatInRange` -30.0 30.0) (`KismetMathLibrary.RandomFloatInRange` -30.0 30.0) 80.0)))))))

(event `SaveInventory`
  (params (PController :type "Controller Object Reference"))
  (bind _playerinventory (`self.PlayerInventory`))
  (bind _asbp_ps_world (cast `/Game/TDS/Blueprints/Game/BP_PS_World` (`Controller.PlayerState` PController)))
  (`/Game/TDS/Blueprints/Game/BP_PS_World.SaveCurrentWeapon` _asbp_ps_world (`TDSInventoryComponent.WeaponInventory` _playerinventory))
  (`/Game/TDS/Blueprints/Game/BP_PS_World.SaveCurrentDiary` _asbp_ps_world (`TDSInventoryComponent.DiaryArray` _playerinventory)))

(event `Key|F`
  (params (Key :type "Key Structure"))
  (:`Pressed`
    (`self.PlayAnimMontage` "/Game/TDS/Assets/Player/Mihail/AM_Mihael_Twist.AM_Mihael_Twist")))

(event `Key|J`
  (params (Key :type "Key Structure")))

(fn `UserConstructionScript`
  (bind _cameraarm (`self.CameraArm`))
  (set `SpringArmComponent.TargetArmLength` (`self.CameraHieght`) _cameraarm)
  (set `SpringArmComponent.bEnableCameraLag` (`self.CameraLag?`) _cameraarm)
  (set `SpringArmComponent.CameraLagSpeed` (`self.CameraLagSpeed`) _cameraarm)
  (`SceneComponent.K2_SetRelativeRotation` _cameraarm (`self.CameraRotation`) false false))