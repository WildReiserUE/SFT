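; BP_TDSInteractable is a world item that lifts and then flies to the player's left hand when clicked.
; A click from BPInteractor plays Timeline_Up to raise the item from its starting Z.
; A looping timer then moves it a hundredth of the remaining distance toward LeftHandSocket each tick, easing in until within 10 units.
; The timer interval scales with the initial distance; the item is never attached.
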(event `self.ReceiveBeginPlay`
  (add `/Game/TDS/Blueprints/ActorComponents/BP_Interactor.BPClicked` (`self.BP_Interactor`) (delegate `BPClicked_Event_0`)))

(event `BPClicked_Event_0`
  (bind (_returnvalue_x _returnvalue_y _returnvalue_z) (`KismetMathLibrary.BreakVector` (`self.K2_GetActorLocation`)))
  (set `self.StartZ` _returnvalue_z)
  (bind (_direction _z) (`Timeline|Timeline_Up` :!via `PlayFromStart`)
    (:`Update`
      (`self.K2_SetActorLocation` (`KismetMathLibrary.MakeVector` _returnvalue_x _returnvalue_y (+ (`self.StartZ`) _z))))
    (:`Finished`
      (bind _returnvalue (`KismetSystemLibrary.K2_SetTimerDelegate` (delegate `MoveItemToPlayer`) (/ (/ (`KismetMathLibrary.VSize` (- (`self.GetSocketLocation`) (`self.K2_GetActorLocation`))) 100.0) 1500.0) true))
      (set `self.TimerMove` _returnvalue))))

(event `MoveItemToPlayer`
  (bind _returnvalue (`self.K2_GetActorLocation`))
  (bind _returnvalue_2 (`self.GetSocketLocation`))
  (bind _returnvalue_3 (- _returnvalue_2 (`self.K2_GetActorLocation`)))
  (if (<= (`KismetMathLibrary.VSize` (- _returnvalue _returnvalue_2)) 10.0)
    (`KismetSystemLibrary.K2_ClearAndInvalidateTimerHandle` (`self.TimerMove`))
    (else
      (`self.K2_SetActorLocation` (+ (* (`KismetMathLibrary.Normal` _returnvalue_3 0.01) (/ (`KismetMathLibrary.VSize` _returnvalue_3) 100.0)) _returnvalue)))))

(fn `GetSocketLocation`
  (returns (ReturnValue :type "Vector Structure"))
  (bind _mesh (`Character.Mesh` (`GameplayStatics.GetPlayerCharacter` 0)))
  (return (`SkeletalMeshSocket.GetSocketLocation` (`SkeletalMesh.FindSocket` (`SkinnedMeshComponent.SkeletalMesh` _mesh) "LeftHandSocket") _mesh)))

(fn `UserConstructionScript`)