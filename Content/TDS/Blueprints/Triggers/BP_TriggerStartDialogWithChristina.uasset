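; Trigger volume in the 03 world level that sets up the dialog with Christina once combat is over.
; Player overlap sets a flag and makes the collision ignore all channels, so it fires once.
; Tick then polls until enemies are dead, Christina is valid and the player is alive.
; It then ends the game mode's sound, shows the "approach the stranger" mission and calls Christina's talk message.
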(event `self.CollisionComponent.OnComponentBeginOverlap`
  (params (OverlappedComponent :type "PrimitiveComponent Object Reference") (OtherActor :type "Actor Object Reference") (OtherComp :type "PrimitiveComponent Object Reference") (OtherBodyIndex :type Integer) (bFromSweep :type Boolean) (SweepResult :type "HitResult Structure (by ref)"))
  (cast `/Game/TDS/Blueprints/Character/BP_PlayerCharacter` OtherActor)
  (set `self.IsCharacterFounded` true)
  (`PrimitiveComponent.SetCollisionResponseToAllChannels` (`self.CollisionComponent`) "ECR_Ignore"))

(event `self.ReceiveTick`
  (params (DeltaSeconds :type "Float (single-precision)"))
  (if (`self.IsCharacterFounded`)
    (bind _asbp_pc_world (cast `/Game/TDS/Blueprints/Game/BP_PC_03World` (`GameplayStatics.GetPlayerController` 0)))
    (bind _asbp_player_character (cast `/Game/TDS/Blueprints/Character/BP_PlayerCharacter` (`Controller.K2_GetPawn` _asbp_pc_world)))
    (bind _output_get (set `self.As BP PC World` _asbp_pc_world))
    (if (and (`TDSPlayerController.EnemyIsDead` _asbp_pc_world) (`KismetSystemLibrary.IsValid` (`self.Christina`)) (`TDSCharacter.bIsALive` _asbp_player_character))
      (set `self.IsCharacterFounded` false)
      (bind _asbp_gm_world (cast `/Game/TDS/Blueprints/Game/BP_GM_03World` (`GameplayStatics.GetGameMode`)))
      (`/Game/TDS/Blueprints/Game/BP_GM_03World.EndSound` _asbp_gm_world)
      (`/Game/TDS/UI/UI_03_Game/W_GameMain.OnShowMission` (`/Game/TDS/Blueprints/Game/BP_PC_03World.W_GameWidget` _output_get) (`self.Подойдите к незнакомке`))
      (message `/Game/TDS/Blueprints/Interfaces/BI_Collision.TalkWithChristina` (`self.Christina`)))))

(fn `UserConstructionScript`)