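; Sliding double door that the player opens by striking its panel with the wrench.
; Inside and sphere overlaps toggle no-key, broken and attack-prompt widgets based on whether the player carries the wrench.
; The sphere binds to the wrench's attack overlap; a single hit covering the panel's Health destroys it, triggering effects and a timeline slide.
; Entering the outside box while open plays a reverse timeline, then resets the panel.
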(event `self.ReceiveBeginPlay`
  (`SceneComponent.SetVisibility` (`self.WidgetUseAttack`) false false)
  (set `self.bDestroed` false))

(event `self.BoxInside.OnComponentBeginOverlap`
  (params (OverlappedComponent :type "PrimitiveComponent Object Reference") (OtherActor :type "Actor Object Reference") (OtherComp :type "PrimitiveComponent Object Reference") (OtherBodyIndex :type Integer) (bFromSweep :type Boolean) (SweepResult :type "HitResult Structure (by ref)"))
  (bind _widgetnokey (`self.WidgetNoKey`))
  (bind _widgetbroken (`self.WidgetBroken`))
  (bind _asbp_player_character (cast `/Game/TDS/Blueprints/Character/BP_PlayerCharacter` OtherActor))
  (bind _weaponinventory (`TDSInventoryComponent.WeaponInventory` (`TDSCharacter.PlayerInventory` _asbp_player_character)))
  (bind _returnvalue (`KismetArrayLibrary.Array_IsValidIndex` _weaponinventory (`KismetArrayLibrary.Array_Find` _weaponinventory "/Game/TDS/Blueprints/Weapon/BP_Weapon_Wrench.BP_Weapon_Wrench_C")))
  (if _returnvalue
    (set `self.bPlayerFindKey` _returnvalue)
    (if (not (`self.bDestroed`))
      (`SceneComponent.SetVisibility` _widgetbroken true false)
      (elif (`SceneComponent.IsVisible` _widgetnokey)
        (`SceneComponent.SetVisibility` _widgetbroken false false)
        (`SceneComponent.SetVisibility` _widgetnokey false false)))
    (else
      (`AudioComponent.Play` (`self.False_Cue`) 0.0)
      (`SceneComponent.SetVisibility` _widgetnokey true false))))

(event `StartMove`
  (bind (_relativelocation_x _relativelocation_y _relativelocation_z) (`KismetMathLibrary.BreakVector` (`SceneComponent.RelativeLocation` (`self.LeftDoor`))))
  (bind (_relativelocation_x_2 _relativelocation_y_2 _relativelocation_z_2) (`KismetMathLibrary.BreakVector` (`SceneComponent.RelativeLocation` (`self.RightDoor`))))
  (if (not (`self.bIsOpen?`))
    (set `self.LocLeftDoor` _relativelocation_x)
    (set `self.LocRightDoor` _relativelocation_x_2)
    (if (not (`SceneComponent.IsVisible` (`self.WidgetNoKey`)))
      (`PrimitiveComponent.SetCollisionEnabled` (`self.BoxInside`) "NoCollision")
      (`AudioComponent.Play` (`self.MoveSound`) 0.0)
      (set `self.bIsOpen?` true)
      (bind (_direction _deltax) (`Timeline|OpenTimer`)
        (:`Update`
          (bind _returnvalue (- (`self.LocLeftDoor`) _deltax))
          (`SceneComponent.K2_SetRelativeLocation` (`self.LeftDoor`) (`KismetMathLibrary.MakeVector` _returnvalue _relativelocation_y _relativelocation_z) false false)
          (bind _returnvalue_2 (+ (`self.LocRightDoor`) _deltax))
          (`SceneComponent.K2_SetRelativeLocation` (`self.RightDoor`) (`KismetMathLibrary.MakeVector` _returnvalue_2 _relativelocation_y_2 _relativelocation_z_2) false false))
        (:`Finished`
          (set `self.LocLeftDoor` _returnvalue)
          (`ActorComponent.Deactivate` (`self.ParticleSystem`))
          (set `self.LocRightDoor` _returnvalue_2))))))

(event `self.BoxOutside.OnComponentBeginOverlap`
  (params (OverlappedComponent :type "PrimitiveComponent Object Reference") (OtherActor :type "Actor Object Reference") (OtherComp :type "PrimitiveComponent Object Reference") (OtherBodyIndex :type Integer) (bFromSweep :type Boolean) (SweepResult :type "HitResult Structure (by ref)"))
  (bind _leftdoor (`self.LeftDoor`))
  (bind _rightdoor (`self.RightDoor`))
  (bind (_relativelocation_x _relativelocation_y _relativelocation_z) (`KismetMathLibrary.BreakVector` (`SceneComponent.RelativeLocation` _leftdoor)))
  (bind (_relativelocation_x_2 _relativelocation_y_2 _relativelocation_z_2) (`KismetMathLibrary.BreakVector` (`SceneComponent.RelativeLocation` _rightdoor)))
  (cast `/Game/TDS/Blueprints/Character/BP_PlayerCharacter` OtherActor)
  (if (`self.bIsOpen?`)
    (`AudioComponent.Play` (`self.MoveSound`) 0.0)
    (bind (_direction _deltax) (`Timeline|Rreverse`)
      (:`Update`
        (bind _returnvalue (+ (`self.LocLeftDoor`) _deltax))
        (`SceneComponent.K2_SetRelativeLocation` _leftdoor (`KismetMathLibrary.MakeVector` _returnvalue _relativelocation_y _relativelocation_z) false false)
        (bind _returnvalue_2 (- (`self.LocRightDoor`) _deltax))
        (`SceneComponent.K2_SetRelativeLocation` _rightdoor (`KismetMathLibrary.MakeVector` _returnvalue_2 _relativelocation_y_2 _relativelocation_z_2) false false))
      (:`Finished`
        (set `self.LocLeftDoor` _returnvalue)
        (set `self.LocRightDoor` _returnvalue_2)
        (set `self.bIsOpen?` false)
        (`PrimitiveComponent.SetCollisionEnabled` (`self.BoxInside`) "QueryAndPhysics")
        (`self.Reset`)))))

(event `self.BoxInside.OnComponentEndOverlap`
  (params (OverlappedComponent :type "PrimitiveComponent Object Reference") (OtherActor :type "Actor Object Reference") (OtherComp :type "PrimitiveComponent Object Reference") (OtherBodyIndex :type Integer))
  (bind _widgetnokey (`self.WidgetNoKey`))
  (bind _widgetbroken (`self.WidgetBroken`))
  (cast `/Game/TDS/Blueprints/Character/BP_PlayerCharacter` OtherActor)
  (if (`SceneComponent.IsVisible` _widgetnokey)
    (`SceneComponent.SetVisibility` _widgetnokey false false)
    (elif (and (not (`self.bDestroed`)) (`SceneComponent.IsVisible` _widgetbroken))
      (`SceneComponent.SetVisibility` _widgetbroken false false))))

(event `self.Sphere.OnComponentBeginOverlap`
  (params (OverlappedComponent :type "PrimitiveComponent Object Reference") (OtherActor :type "Actor Object Reference") (OtherComp :type "PrimitiveComponent Object Reference") (OtherBodyIndex :type Integer) (bFromSweep :type Boolean) (SweepResult :type "HitResult Structure (by ref)"))
  (bind _widgetuseattack (`self.WidgetUseAttack`))
  (bind _bplayerfindkey (`self.bPlayerFindKey`))
  (`|ExecutionSequence`
    (:`then_0`
      (cast `/Game/TDS/Blueprints/Character/BP_PlayerCharacter` OtherActor)
      (if _bplayerfindkey
        (if (not (and (`SceneComponent.IsVisible` _widgetuseattack) _bplayerfindkey))
          (`SceneComponent.SetVisibility` _widgetuseattack true false))))
    (:`then_1`
      (bind _asbp_weapon_wrench (cast `/Game/TDS/Blueprints/Weapon/BP_Weapon_Wrench` OtherActor))
      (bind _attackspherecomponent (`TDSWeaponBase.AttackSphereComponent` _asbp_weapon_wrench))
      (if (and (`KismetSystemLibrary.IsValid` _attackspherecomponent) (not (`self.bDestroed`)))
        (add `PrimitiveComponent.OnComponentBeginOverlap` _attackspherecomponent (delegate `OnComponentBeginOverlap_Event_0`))))))

(event `OnComponentBeginOverlap_Event_0`
  (params (OverlappedComponent :type "PrimitiveComponent Object Reference") (OtherActor :type "Actor Object Reference") (OtherComp :type "PrimitiveComponent Object Reference") (OtherBodyIndex :type Integer) (bFromSweep :type Boolean) (SweepResult :type "HitResult Structure (by ref)"))
  (remove `PrimitiveComponent.OnComponentBeginOverlap` (`TDSWeaponBase.AttackSphereComponent` (stale `self.Sphere.OnComponentBeginOverlap` _asbp_weapon_wrench)) (delegate `OnComponentBeginOverlap_Event_0`))
  (`/Engine/EditorBlueprintResources/StandardMacros.DoOnce` false :!label _label
    (:`Completed`
      (if (<= (- (`self.Health`) (`.WeaponDamage` (break `WeaponSettings` (`TDSWeaponBase.WeaponInfo` (stale `self.Sphere.OnComponentBeginOverlap` _asbp_weapon_wrench))))) 0.0)
        (set `self.bDestroed` true)
        (`AudioComponent.Play` (`self.Audio`) 0.0)
        (`SceneComponent.SetVisibility` (`self.WidgetUseAttack`) false false)
        (`PrimitiveComponent.SetRenderCustomDepth` (`self.Panel`) false)
        (`ActorComponent.Activate` (`self.ParticleSystem`) true)
        (`self.StartMove`)))))

(event `Reset`
  (`PrimitiveComponent.SetRenderCustomDepth` (`self.Panel`) true)
  (`ActorComponent.Deactivate` (`self.ParticleSystem`))
  (set `self.Health` 40.0)
  (set `self.bDestroed` false)
  (goto _label :!via `Reset`))

(event `self.Sphere.OnComponentEndOverlap`
  (params (OverlappedComponent :type "PrimitiveComponent Object Reference") (OtherActor :type "Actor Object Reference") (OtherComp :type "PrimitiveComponent Object Reference") (OtherBodyIndex :type Integer))
  (bind _widgetuseattack (`self.WidgetUseAttack`))
  (cast `/Game/TDS/Blueprints/Character/BP_PlayerCharacter` OtherActor)
  (if (`SceneComponent.IsVisible` _widgetuseattack)
    (`SceneComponent.SetVisibility` _widgetuseattack false false)))

(fn `UserConstructionScript`)