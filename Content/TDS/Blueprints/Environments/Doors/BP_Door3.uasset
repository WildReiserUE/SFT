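; BP_Door3 is a sliding door that responds to the player character once the level's enemy condition allows it.
; OpenDoor calls OnCloseMission on the BP_PC_03World controller's game widget and sets the can-open flag from EnemyIsDead.
; While that flag is set, overlapping either trigger box plays a timeline and leaving reverses it.
; Each timeline update subtracts the track value from the mesh's current relative Z, so offsets accumulate.
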(event `self.Box.OnComponentBeginOverlap`
  (params (OverlappedComponent :type "PrimitiveComponent Object Reference") (OtherActor :type "Actor Object Reference") (OtherComp :type "PrimitiveComponent Object Reference") (OtherBodyIndex :type Integer) (bFromSweep :type Boolean) (SweepResult :type "HitResult Structure (by ref)"))
  (bind _doormesh (`self.DoorMesh`))
  (bind (_relativelocation_x _relativelocation_y _relativelocation_z) (`KismetMathLibrary.BreakVector` (`SceneComponent.RelativeLocation` _doormesh)))
  (cast `/Game/TDS/Blueprints/Character/BP_PlayerCharacter` OtherActor)
  (if (`self.IsCanOperDoor`) :!label _label
    (bind (_direction _newtrack_0) (`Timeline|Timeline_1` :!label _label_2)
      (:`Update`
        (`SceneComponent.K2_SetRelativeLocation` _doormesh (`KismetMathLibrary.MakeVector` _relativelocation_x _relativelocation_y (- _relativelocation_z _newtrack_0)) false false)))))

(event `self.Box1.OnComponentBeginOverlap`
  (params (OverlappedComponent :type "PrimitiveComponent Object Reference") (OtherActor :type "Actor Object Reference") (OtherComp :type "PrimitiveComponent Object Reference") (OtherBodyIndex :type Integer) (bFromSweep :type Boolean) (SweepResult :type "HitResult Structure (by ref)"))
  (cast `/Game/TDS/Blueprints/Character/BP_PlayerCharacter` OtherActor)
  (goto _label))

(event `self.Box.OnComponentEndOverlap`
  (params (OverlappedComponent :type "PrimitiveComponent Object Reference") (OtherActor :type "Actor Object Reference") (OtherComp :type "PrimitiveComponent Object Reference") (OtherBodyIndex :type Integer))
  (cast `/Game/TDS/Blueprints/Character/BP_PlayerCharacter` OtherActor)
  (if (`self.IsCanOperDoor`) :!label _label_3
    (goto _label_2 :!via `Reverse`)))

(event `self.Box1.OnComponentEndOverlap`
  (params (OverlappedComponent :type "PrimitiveComponent Object Reference") (OtherActor :type "Actor Object Reference") (OtherComp :type "PrimitiveComponent Object Reference") (OtherBodyIndex :type Integer))
  (cast `/Game/TDS/Blueprints/Character/BP_PlayerCharacter` OtherActor)
  (goto _label_3))

(event `/Game/TDS/Blueprints/Interfaces/BI_Collision.OpenDoor`
  (bind _as_bp_pc_world (`self.As BP PC World`))
  (bind _asbp_pc_03world (cast `/Game/TDS/Blueprints/Game/BP_PC_03World` (`GameplayStatics.GetPlayerController` 0)))
  (bind _output_get (set `self.As BP PC World` _asbp_pc_03world))
  (`/Engine/EditorBlueprintResources/StandardMacros.IsValid` _output_get
    (:`Is Valid`
      (`/Game/TDS/UI/UI_03_Game/W_GameMain.OnCloseMission` (`/Game/TDS/Blueprints/Game/BP_PC_03World.W_GameWidget` _as_bp_pc_world))
      (set `self.IsCanOperDoor` (`TDSPlayerController.EnemyIsDead` _as_bp_pc_world)))))

(fn `UserConstructionScript`)