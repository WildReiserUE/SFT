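; BP_Bereza is a birch tree tutorial interactable where the player receives a health bottle.
; Its overlap sphere toggles the pickup flag on the player's inventory and shows a widget, with a return-to-birch mission prompt on leaving early.
; The inventory's OnReceiveItem delegate, bound at BeginPlay, shows the bottle and healing hint through the player controller's game widget and flags the tutorial step finished.
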(event `self.ReceiveBeginPlay`
  (bind _returnvalue (`self.GetComponentByClass` (`GameplayStatics.GetPlayerPawn` 0) "/Script/TDS.TDSInventoryComponent"))
  (if (`KismetSystemLibrary.IsValid` _returnvalue)
    (add `TDSInventoryComponent.OnReceiveItem` _returnvalue (delegate `OnPressed_E`))))

(event `OnPressed_E`
  (bind _asbp_pc_03world (cast `/Game/TDS/Blueprints/Game/BP_PC_03World` (`GameplayStatics.GetPlayerController` 0)))
  (`/Engine/EditorBlueprintResources/StandardMacros.IsValid` _asbp_pc_03world
    (:`Is Valid`
      (bind _w_gamewidget (`/Game/TDS/Blueprints/Game/BP_PC_03World.W_GameWidget` _asbp_pc_03world))
      ;[1 1 1] Конец туториала смотри в контроллере
      (`/Game/TDS/UI/UI_03_Game/W_GameMain.OnShowBottle` _w_gamewidget)
      (`/Game/TDS/UI/UI_03_Game/W_GameMain.OnShowMission` _w_gamewidget "Нажмите \"Т\" для пополнения здоровья")
      (set `self.FinishedTutorial` true))))

(event `self.SphereComponent.OnComponentBeginOverlap`
  (params (OverlappedComponent :type "PrimitiveComponent Object Reference") (OtherActor :type "Actor Object Reference") (OtherComp :type "PrimitiveComponent Object Reference") (OtherBodyIndex :type Integer) (bFromSweep :type Boolean) (SweepResult :type "HitResult Structure (by ref)"))
  (cast `/Game/TDS/Blueprints/Game/BP_PC_03World` (`GameplayStatics.GetPlayerController` 0))
  (bind _asbp_player_character (cast `/Game/TDS/Blueprints/Character/BP_PlayerCharacter` OtherActor))
  (set `TDSInventoryComponent.bIsCanPickupTo` true (`TDSCharacter.PlayerInventory` _asbp_player_character))
  (set `self.FinishedSwitch` true)
  (`SceneComponent.SetVisibility` (`self.Widget`) true false))

(event `self.SphereComponent.OnComponentEndOverlap`
  (params (OverlappedComponent :type "PrimitiveComponent Object Reference") (OtherActor :type "Actor Object Reference") (OtherComp :type "PrimitiveComponent Object Reference") (OtherBodyIndex :type Integer))
  (bind _asbp_player_character (cast `/Game/TDS/Blueprints/Character/BP_PlayerCharacter` OtherActor))
  (bind _asbp_pc_03world (cast `/Game/TDS/Blueprints/Game/BP_PC_03World` (`GameplayStatics.GetPlayerController` 0)))
  (bind _returnvalue (`self.GetComponentByClass` _asbp_player_character "/Script/TDS.TDSInventoryComponent"))
  (if (and (`KismetSystemLibrary.IsValid` _asbp_pc_03world) (`self.FinishedSwitch`) (`KismetSystemLibrary.IsValid` _returnvalue) (not (`self.FinishedTutorial`)))
    (`/Game/TDS/UI/UI_03_Game/W_GameMain.OnShowMission` (`/Game/TDS/Blueprints/Game/BP_PC_03World.W_GameWidget` _asbp_pc_03world) "Вернитесь к березе")
    (`SceneComponent.SetVisibility` (`self.Widget`) false false))
  (set `TDSInventoryComponent.bIsCanPickupTo` false _returnvalue)
  (set `self.FinishedSwitch` false))

(fn `UserConstructionScript`)